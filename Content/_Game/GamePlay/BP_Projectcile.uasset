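; BP_Projectcile is a projectile actor that moves itself every frame.
; Tick sets its location without sweep, adding the current location scaled by MoveSpeed and delta time, so movement follows the world-origin position vector rather than facing.
; BeginPlay saves InitialMoveSpeed, which is never read.
; SpeedBoost is an empty event; its multiply-and-delay logic is disconnected, and its reset assigns MoveSpeed to itself.
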(event EventTick
  (params (DeltaSeconds :type Float%20%28single-precision%29))
  (Transformation|SetActorLocation (+ (* (* DeltaSeconds (Variables|Default|GetMove%20Speed)) (Transformation|GetActorLocation)) (Transformation|GetActorLocation)) false false))

(event EventSpeedBoost
  (params (Multipyer :type Float%20%28double-precision%29) (Duration :type Float%20%28double-precision%29)))

(event EventBeginPlay
  (Variables|Default|Setinitial%20Move%20Speed (Variables|Default|GetMove%20Speed)))

(fn ConstructionScript)